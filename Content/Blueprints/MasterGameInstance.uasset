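; Game instance Blueprint that handles menu display and starting or joining multiplayer games.
; Show events lazily create and cache the main, host, join and settings menu widgets, add them to the viewport, show the cursor and disable input on the controlled pawn.
; HostGame and JoinServer travel through "open" console commands, loading a map as a listen server or connecting to an IP.
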(event Custom|JoinServer
  (params (IP :type String%20%28by%20ref%29))
  ;[1 1 1] Join Server
  (Development|ExecuteConsoleCommand (Utilities|String|ToString(Text) (Utilities|Text|FormatText "open {ip}" IP)) (Game|GetPlayerController 0)))

(event Custom|ShowMainMenu
  (bind _returnvalue (Game|GetPlayerController 0))
  (bind _returnvalue_2 (Game|GetPlayerController 0))
  ;[1 1 1] Show Main Menu
  (Utilities|IsValid (Variables|Default|GetMainMenu%20WB)
    (:Is%20Valid
      _)
    (:Is%20Not%20Valid
      (bind _returnvalue_3 (UserInterface|CreateWidget "/Game/Blueprints/UI/WB_MainMenu.WB_MainMenu_C" _returnvalue))
      (Variables|Default|SetMainMenu%20WB _returnvalue_3)))
  (UserInterface|Viewport|AddtoViewport (Variables|Default|GetMainMenu%20WB) 0)
  (Variables|/Script/Engine.PlayerController|SetbShowMouseCursor _returnvalue true)
  (Input|DisableInput (Pawn|GetControlledPawn _returnvalue_2) _returnvalue_2))

(event Custom|ShowJoinGameMenu
  (bind _returnvalue (Game|GetPlayerController 0))
  (bind _returnvalue_2 (Game|GetPlayerController 0))
  ;[1 1 1] Show Join Game
  (Utilities|IsValid (Variables|Default|GetJoinGameMenu%20WB)
    (:Is%20Valid
      _)
    (:Is%20Not%20Valid
      (bind _returnvalue_3 (UserInterface|CreateWidget "/Game/Blueprints/UI/WB_JoinGameMenu.WB_JoinGameMenu_C" _returnvalue))
      (Variables|Default|SetJoinGameMenu%20WB _returnvalue_3)))
  (UserInterface|Viewport|AddtoViewport (Variables|Default|GetJoinGameMenu%20WB) 0)
  (Variables|/Script/Engine.PlayerController|SetbShowMouseCursor _returnvalue true)
  (Input|DisableInput (Pawn|GetControlledPawn _returnvalue_2) _returnvalue_2))

(event Custom|ShowSettingsMenu
  (bind _returnvalue (Game|GetPlayerController 0))
  (bind _returnvalue_2 (Game|GetPlayerController 0))
  ;[1 1 1] Show Settings
  (Utilities|IsValid (Variables|Default|GetSettingsMenu%20WB)
    (:Is%20Valid
      _)
    (:Is%20Not%20Valid
      (bind _returnvalue_3 (UserInterface|CreateWidget "/Game/Blueprints/UI/WB_SettingsMenu.WB_SettingsMenu_C" _returnvalue))
      (Variables|Default|SetSettingsMenu%20WB _returnvalue_3)))
  (UserInterface|Viewport|AddtoViewport (Variables|Default|GetSettingsMenu%20WB) 0)
  (Variables|/Script/Engine.PlayerController|SetbShowMouseCursor _returnvalue true)
  (Input|DisableInput (Pawn|GetControlledPawn _returnvalue_2) _returnvalue_2))

(event Custom|ShowHostGameMenu
  (bind _returnvalue (Game|GetPlayerController 0))
  (bind _returnvalue_2 (Game|GetPlayerController 0))
  ;[1 1 1] Host New Game
  (Utilities|IsValid (Variables|Default|GetNewGameMenu%20WB)
    (:Is%20Valid
      _)
    (:Is%20Not%20Valid
      (bind _returnvalue_3 (UserInterface|CreateWidget "/Game/Blueprints/UI/WB_NewGameMenu.WB_NewGameMenu_C" _returnvalue_2))
      (Variables|Default|SetNewGameMenu%20WB _returnvalue_3)))
  (UserInterface|Viewport|AddtoViewport (Variables|Default|GetNewGameMenu%20WB) 0)
  (Variables|/Script/Engine.PlayerController|SetbShowMouseCursor _returnvalue_2 true)
  (Input|DisableInput (Pawn|GetControlledPawn _returnvalue) _returnvalue))

(event Custom|HostGame
  (params (MapName :type String))
  ;[1 1 1] Host Game
  (Development|ExecuteConsoleCommand (Utilities|String|ToString(Text) (Utilities|Text|FormatText "open {mapname}?listen" MapName)) (Game|GetPlayerController 0)))