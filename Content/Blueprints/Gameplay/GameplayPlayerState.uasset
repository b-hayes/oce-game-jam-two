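; GameplayPlayerState is a player state that carries kill and death counts with RepNotify for the scoreboard.
; When either value replicates, its OnRep function casts player controller 0 to TopDownController and calls RefreshPlayerList on that controller's ScoreboardWidget, if valid.
; BeginPlay and the construction script are empty.
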(event EventBeginPlay)

(fn ConstructionScript)

(fn OnRepDeaths
  (bind _returnvalue (Game|GetPlayerController 0))
  (Utilities|IsValid _returnvalue
    (:Is%20Valid
      (bind _astop_down_controller (Utilities|Casting|CastToTopDownController _returnvalue))
      (Utilities|IsValid (Variables|/Game/Blueprints/Gameplay/TopDownController.TopDownController_C|GetScoreboardWidget _astop_down_controller)
        (:Is%20Valid
          (Default|RefreshPlayerList (Variables|/Game/Blueprints/Gameplay/TopDownController.TopDownController_C|GetScoreboardWidget _astop_down_controller)))))))

(fn OnRepKills
  (bind _returnvalue (Game|GetPlayerController 0))
  (Utilities|IsValid _returnvalue
    (:Is%20Valid
      (bind _astop_down_controller (Utilities|Casting|CastToTopDownController _returnvalue))
      (Utilities|IsValid (Variables|/Game/Blueprints/Gameplay/TopDownController.TopDownController_C|GetScoreboardWidget _astop_down_controller)
        (:Is%20Valid
          (Default|RefreshPlayerList (Variables|/Game/Blueprints/Gameplay/TopDownController.TopDownController_C|GetScoreboardWidget _astop_down_controller)))))))