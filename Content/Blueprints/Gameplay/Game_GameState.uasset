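; Game state for a kill-based multiplayer match that tracks the first and second place players and relays match flow to local player controllers.
; Score checks rank players by kills, with deaths used in tie-breaks, then the server has the game mode test the leader's kills for a win.
; Game start, the MatchStarted RepNotify and game end trigger the countdown, match begin, and win screen with input disabled on player controller 0.
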(event Custom|EndGameClients
  (params (Winner :type Text) (2ndPlace :type Text))
  (bind _asgame_player_controller (Utilities|Casting|CastToGame_PlayerController (Game|GetPlayerController 0)))
  (Default|ShowWinScreen _asgame_player_controller Winner 2ndPlace)
  (Input|DisableInput _asgame_player_controller _asgame_player_controller))

(event Custom|CheckPlayersScores
  (params (PlayerState :type Game%20Player%20State%20Object%20Reference) (Kills :type Integer) (Deaths :type Integer))
  ;[1 1 1] Check who is currently leading
  (CallFunction|CaclulateFirstandSecondPlace PlayerState Kills Deaths)
  (if (Networking|IsServer)
    (bind _asgame_game_mode (Utilities|Casting|CastToGame_GameMode (Game|GetGameMode)))
    (Default|CheckKillsWinCondition _asgame_game_mode (Variables|Default|GetFirstPlaceKills))))

(event Custom|MulticastGameStart
  (bind _asgame_player_controller (Utilities|Casting|CastToGame_PlayerController (Game|GetPlayerController 0)))
  (Default|ShowCountdown _asgame_player_controller))

(event EventBeginPlay)

(event EventTick
  (params (DeltaSeconds :type Float%20%28single-precision%29)))

(fn ConstructionScript)

(fn OnRepFirstPlacePlayer)

(fn OnRepSecondPlacePlayer)

(fn CaclulateFirstandSecondPlace
  (params (Player :type Game%20Player%20State%20Object%20Reference) (PlayerKills :type Integer) (PlayerDeaths :type Integer))
  (Utilities|IsValid (Variables|Default|GetFirstPlacePlayer)
    (:Is%20Valid
      (if (> PlayerKills (Variables|Default|GetFirstPlaceKills))
        (Variables|Default|SetSecondPlacePlayer (Variables|Default|GetFirstPlacePlayer) :!label _label)
        (Variables|Default|SetSecondPlaceKills (Variables|Default|GetFirstPlaceKills))
        (Variables|Default|SetSecondPlaceDeaths (Variables|Default|GetFirstPlaceDeaths))
        (Variables|Default|SetFirstPlacePlayer Player :!label _label_2)
        (Variables|Default|SetFirstPlaceKills PlayerKills :!label _label_3)
        (Variables|Default|SetFirstPlaceDeaths PlayerDeaths)
        (else
          (Utilities|IsValid (Variables|Default|GetSecondPlacePlayer)
            (:Is%20Valid
              (if (== PlayerKills (Variables|Default|GetFirstPlaceKills))
                (if (< PlayerDeaths (Variables|Default|GetFirstPlaceDeaths))
                  (if (== Player (Variables|Default|GetFirstPlacePlayer))
                    (goto _label)
                    (else
                      (goto _label_3)))
                  (else
                    (if (< PlayerDeaths (Variables|Default|GetSecondPlaceDeaths)) :!label _label_4
                      (Variables|Default|SetSecondPlacePlayer Player :!label _label_5)
                      (Variables|Default|SetSecondPlaceKills PlayerKills)
                      (Variables|Default|SetSecondPlaceDeaths PlayerDeaths))))
                (elif (> PlayerDeaths (Variables|Default|GetSecondPlaceKills))
                  (goto _label_5)
                  (else
                    (goto _label_4)))))
            (:Is%20Not%20Valid
              (goto _label_5))))))
    (:Is%20Not%20Valid
      (goto _label_2))))

(fn OnRepMatchStarted
  (bind _asgame_player_controller (Utilities|Casting|CastToGame_PlayerController (Game|GetPlayerController 0)))
  (Default|MatchBegin _asgame_player_controller))