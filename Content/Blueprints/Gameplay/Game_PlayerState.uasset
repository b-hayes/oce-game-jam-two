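; Player state that carries replicated Kills and Deaths stats for the scoreboard.
; Each stat's RepNotify fetches the first local player controller, casts it to Game_PlayerController and tells its ScoreboardWidget, when valid, to refresh the player list.
; The blueprint has no other active logic, so this file only reacts to stat changes and does not modify them.
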(event EventBeginPlay)

(fn ConstructionScript)

(fn OnRepDeaths
  (bind _returnvalue (Game|GetPlayerController 0))
  (Utilities|IsValid _returnvalue
    (:Is%20Valid
      (bind _asgame_player_controller (Utilities|Casting|CastToGame_PlayerController _returnvalue))
      (Utilities|IsValid (Variables|/Game/Blueprints/Gameplay/Game_PlayerController.Game_PlayerController_C|GetScoreboardWidget _asgame_player_controller)
        (:Is%20Valid
          (Default|RefreshPlayerList (Variables|/Game/Blueprints/Gameplay/Game_PlayerController.Game_PlayerController_C|GetScoreboardWidget _asgame_player_controller)))))))

(fn OnRepKills
  (bind _returnvalue (Game|GetPlayerController 0))
  (Utilities|IsValid _returnvalue
    (:Is%20Valid
      (bind _asgame_player_controller (Utilities|Casting|CastToGame_PlayerController _returnvalue))
      (Utilities|IsValid (Variables|/Game/Blueprints/Gameplay/Game_PlayerController.Game_PlayerController_C|GetScoreboardWidget _asgame_player_controller)
        (:Is%20Valid
          (Default|RefreshPlayerList (Variables|/Game/Blueprints/Gameplay/Game_PlayerController.Game_PlayerController_C|GetScoreboardWidget _asgame_player_controller)))))))