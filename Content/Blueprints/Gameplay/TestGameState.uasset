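; Game state that tracks the top two players of a kill-based match and triggers the end-of-game screen.
; CheckIfLeader compares a player's kills and deaths against the stored first and second place entries, updating player references and scores.
; The two place references have RepNotify functions, both empty.
; EndGameClients passes winner and runner-up to the first Game_PlayerController's win screen, then disables its input.
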(event Custom|EndGameClients
  (params (Winner :type Text) (2ndPlace :type Text))
  (bind _asgame_player_controller (Utilities|Casting|CastToGame_PlayerController (Game|GetPlayerController 0)))
  (Default|ShowWinScreen _asgame_player_controller Winner 2ndPlace)
  (Input|DisableInput _asgame_player_controller _asgame_player_controller))

(event Custom|CheckIfLeader
  (params (PlayerState :type Game%20Player%20State%20Object%20Reference) (Kills :type Integer) (Deaths :type Integer))
  (Utilities|IsValid (Variables|Default|GetFirstPlacePlayer)
    (:Is%20Valid
      (if (> Kills (Variables|Default|GetFirstPlaceKills))
        (Variables|Default|SetSecondPlacePlayer (Variables|Default|GetFirstPlacePlayer) :!label _label)
        (Variables|Default|SetSecondPlaceKills (Variables|Default|GetFirstPlaceKills))
        (Variables|Default|SetSecondPlaceDeaths (Variables|Default|GetFirstPlaceDeaths))
        (Variables|Default|SetFirstPlacePlayer PlayerState :!label _label_2)
        (Variables|Default|SetFirstPlaceKills Kills :!label _label_3)
        (Variables|Default|SetFirstPlaceDeaths Deaths)
        (else
          (Utilities|IsValid (Variables|Default|GetSecondPlacePlayer)
            (:Is%20Valid
              (if (== Kills (Variables|Default|GetFirstPlaceKills))
                (if (< Deaths (Variables|Default|GetFirstPlaceDeaths))
                  (if (== PlayerState (Variables|Default|GetFirstPlacePlayer))
                    (goto _label)
                    (else
                      (goto _label_3)))
                  (else
                    (if (< Deaths (Variables|Default|GetSecondPlaceDeaths)) :!label _label_4
                      (Variables|Default|SetSecondPlacePlayer PlayerState :!label _label_5)
                      (Variables|Default|SetSecondPlaceKills Kills)
                      (Variables|Default|SetSecondPlaceDeaths Deaths))))
                (elif (> Kills (Variables|Default|GetSecondPlaceKills))
                  (goto _label_5)
                  (else
                    (goto _label_4)))))
            (:Is%20Not%20Valid
              (goto _label_5))))))
    (:Is%20Not%20Valid
      (goto _label_2))))

(event EventBeginPlay)

(event EventTick
  (params (DeltaSeconds :type Float%20%28single-precision%29)))

(fn ConstructionScript)

(fn OnRepFirstPlacePlayer)

(fn OnRepSecondPlacePlayer)