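; Ability component for a TopDownCharacter that fires its current single-use ability, either Proximity Mine or Rail Gun, then clears it.
; The mine spawns at the ground point found by a downward trace, tagged with the activating player controller.
; The rail gun sphere-traces forward for pawns, damages the characters hit, then multicasts a sound and beam effect.
; CurrentAbility has an empty OnRep, and DestroyAbility removes the component.
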(event Custom|ActivateAbility
  (switch Utilities|FlowControl|Switch|SwitchonPickupAbilities (Variables|Default|GetCurrentAbility)
    (:NewEnumerator1
      (CallFunction|ActivateProximityMine))
    (:NewEnumerator3
      (CallFunction|ActivateRailGun)))
  (Variables|Default|SetCurrentAbility "NewEnumerator2"))

(event Custom|DestroyAbility
  (Components|DestroyComponent))

(event Custom|RailGunMulticast
  (params (StartLocation :type Vector) (EndLocation :type Vector))
  (Audio|SpawnSoundatLocation "/Game/Audio/SFX/512469__michael-grinnell__laser-shot.512469__michael-grinnell__laser-shot" StartLocation "0, 0, 0" 1.0 1.0 0.0 0 0)
  (bind _returnvalue (Niagara|SpawnSystematLocation "/Game/Blueprints/Particles/RailGun_System.RailGun_System" StartLocation))
  (Effects|Components|ParticleSystem|SetVectorParameter _returnvalue "End" EndLocation))

(event EventBeginPlay)

(event EventTick
  (params (DeltaSeconds :type Float%20%28single-precision%29)))

(fn OnRepCurrentAbility)

(fn ActivateProximityMine
  (bind _astop_down_character (Utilities|Casting|CastToTopDownCharacter (Components|GetOwner)))
  (bind _outhit (Collision|LineTraceForObjects (Transformation|GetActorLocation _astop_down_character) (- (Transformation|GetActorLocation _astop_down_character) "0, 0,1000.000000") (Utilities|Array|MakeArray "ObjectTypeQuery1") false (Utilities|Array|MakeArray 0) "None"))
  (bind _asplayer_controller (Utilities|Casting|CastToPlayerController (Pawn|GetController _astop_down_character)))
  (Game|SpawnActorfromClass "/Game/Blueprints/Actors/ProximityMine.ProximityMine_C" (Math|Transform|MakeTransform (.ImpactPoint (Collision|BreakHitResult _outhit)) "0, 0, 0" "1,1,1") "Undefined" 0 _asplayer_controller self))

(fn ActivateRailGun
  (bind _astop_down_character (Utilities|Casting|CastToTopDownCharacter (Components|GetOwner)))
  (bind _outhits (Collision|MultiSphereTraceForObjects (Transformation|GetActorLocation _astop_down_character) (+ (Transformation|GetActorLocation _astop_down_character) (* (Math|Vector|GetForwardVector (Transformation|GetActorRotation _astop_down_character)) 1e+04)) 0.0 (Utilities|Array|MakeArray "ObjectTypeQuery3") false 0 "None"))
  (bind _asgame_player_controller (Utilities|Casting|CastToGame_PlayerController (Pawn|GetController _astop_down_character)))
  (for _array_element _outhits
    (bind _astop_down_character_2 (Utilities|Casting|CastToTopDownCharacter (.HitActor (Collision|BreakHitResult _array_element))))
    (Default|DamageCharacter _astop_down_character_2 5 _asgame_player_controller (Transformation|GetWorldLocation (Variables|/Game/Blueprints/Character/TopDownCharacter.TopDownCharacter_C|GetGunEnd _astop_down_character))))
  (CallFunction|RailGunMulticast (Transformation|GetWorldLocation (Variables|/Game/Blueprints/Character/TopDownCharacter.TopDownCharacter_C|GetGunEnd _astop_down_character)) (+ (Transformation|GetActorLocation _astop_down_character) (* (Math|Vector|GetForwardVector (Transformation|GetActorRotation _astop_down_character)) 1e+04))))