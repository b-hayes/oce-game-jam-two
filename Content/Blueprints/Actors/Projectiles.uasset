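; Projectile actor for a top-down multiplayer shooter that bounces off surfaces and damages characters on hit.
; On the server, an overlap with any character other than its instigator deals damage credited to the shooting player controller, then destroys it.
; Bounces play effects and pitch-randomized sound, while the server counts them and destroys the projectile after a few or when it stops.
; A launch sound plays on spawn.
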(event OnComponentBeginOverlap(Sphere1)
  (params (OverlappedComponent :type Primitive%20Component%20Object%20Reference) (OtherActor :type Actor%20Object%20Reference) (OtherComp :type Primitive%20Component%20Object%20Reference) (OtherBodyIndex :type Integer) (bFromSweep :type Boolean) (SweepResult :type Hit%20Result%20Structure%20%28by%20ref%29))
  (Networking|SwitchHasAuthority
    (:Authority
      ;[1 1 1] Shoot self disabled
      (if (not (== (Game|GetInstigator) OtherActor))
        (bind _astop_down_character (Utilities|Casting|CastToTopDownCharacter OtherActor))
        (Default|DamageCharacter _astop_down_character 1 (Variables|Default|GetPlayerWhoShot) (.ImpactPoint (Collision|BreakHitResult SweepResult)))
        (Actor|DestroyActor)))))

(event OnProjectileBounce(ProjectileMovement)
  (params (ImpactResult :type Hit%20Result%20Structure%20%28by%20ref%29) (ImpactVelocity :type Vector%20%28by%20ref%29 :default "0, 0, 0"))
  (bind _location (Collision|BreakHitResult ImpactResult))
  (Niagara|SpawnSystematLocation "/Game/Blueprints/Particles/Bounce_System.Bounce_System" _location)
  (Audio|PlaySoundatLocation "/Game/Audio/SFX/523088__magnuswaker__energy-bounce-1.523088__magnuswaker__energy-bounce-1" _location "0, 0, 0" 1.0 (Math|Random|RandomFloatinRange 1.5 2.1) 0.0 "/Game/Audio/Settings/MediumSounds.MediumSounds" 0 0)
  (Networking|SwitchHasAuthority
    (:Authority
      (if (> (Variables|Default|GetBounceNumber) 1)
        (Actor|DestroyActor)
        (else
          (Math|Integer|IncrementInt (Variables|Default|GetBounceNumber)))))))

(event OnProjectileStop(ProjectileMovement)
  (params (ImpactResult :type Hit%20Result%20Structure%20%28by%20ref%29))
  (Networking|SwitchHasAuthority
    (:Authority
      (Actor|DestroyActor))))

(event EventBeginPlay
  (Audio|PlaySoundatLocation "/Game/Audio/SFX/flaunch.flaunch" (Transformation|GetActorLocation) "0, 0, 0" 1.0 1.0 0.0 "/Game/Audio/Settings/MediumSounds.MediumSounds" 0 0))

(event Collision|EventActorBeginOverlap
  (params (OtherActor :type Actor%20Object%20Reference)))

(fn ConstructionScript)