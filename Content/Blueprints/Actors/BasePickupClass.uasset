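; Base pickup actor for the top-down game that grants an ability to the character that overlaps it, playing a sound on spawn.
; On server overlap, PickupCondition checks the character's current ability against a specific enum value before DoAbility, an empty hook, and GrantItem run.
; GrantItem assigns AbilityToGrant once with authority and restarts the owning PickupStand's spawn timer.
; The pickup then hides and destroys itself after a short delay.
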(event OnComponentBeginOverlap(Sphere)
  (params (OverlappedComponent :type Primitive%20Component%20Object%20Reference) (OtherActor :type Actor%20Object%20Reference) (OtherComp :type Primitive%20Component%20Object%20Reference) (OtherBodyIndex :type Integer) (bFromSweep :type Boolean) (SweepResult :type Hit%20Result%20Structure%20%28by%20ref%29)))

(event Custom|DoAbility
  (params (Actor :type Actor%20Object%20Reference)))

(event Custom|GrantItem
  (params (Actor :type Actor%20Object%20Reference))
  (bind _astop_down_character (Utilities|Casting|CastToTopDownCharacter Actor))
  (Utilities|FlowControl|DoOnce false
    (:Completed
      (Networking|SwitchHasAuthority
        (:Authority
          (Variables|/Game/Blueprints/Components/AbilityComponent.AbilityComponent_C|SetCurrentAbility (Variables|/Game/Blueprints/Character/TopDownCharacter.TopDownCharacter_C|GetAbilityBase _astop_down_character) (Variables|Default|GetAbilityToGrant))
          (bind _aspickup_stand (Utilities|Casting|CastToPickupStand (Components|GetOwner)))
          (Default|StartItemSpawnTimer _aspickup_stand))))))

(event Custom|PickedUp
  (Rendering|SetActorHiddenInGame true))

(event EventBeginPlay
  (Audio|SpawnSoundatLocation "/Game/Audio/SFX/478336__joao-janz__bouncing-power-up-1-3.478336__joao-janz__bouncing-power-up-1-3" (Transformation|GetWorldLocation (Variables|Default|GetSphere)) "0, 0, 0" 1.0 1.0 0.0 "/Game/Audio/Settings/CloseSounds.CloseSounds" 0))

(event Collision|EventActorBeginOverlap
  (params (OtherActor :type Actor%20Object%20Reference))
  (if (Networking|IsServer)
    (bind _canpickup (CallFunction|PickupCondition))
    (if _canpickup
      (CallFunction|DoAbility OtherActor)
      (CallFunction|GrantItem OtherActor)
      (CallFunction|PickedUp)
      (Utilities|FlowControl|Delay 1.0)
      (Actor|DestroyActor))))

(event EventTick
  (params (DeltaSeconds :type Float%20%28single-precision%29)))

(fn ConstructionScript)

(fn PickupCondition
  (params (Actor :type Actor%20Object%20Reference))
  (bind _astop_down_character (Utilities|Casting|CastToTopDownCharacter Actor))
  (return (Utilities|Enum|Equal(Enum) (Variables|/Game/Blueprints/Components/AbilityComponent.AbilityComponent_C|GetCurrentAbility (Actor|GetComponentbyClass _astop_down_character "/Game/Blueprints/Components/AbilityComponent.AbilityComponent_C")) "NewEnumerator2")))