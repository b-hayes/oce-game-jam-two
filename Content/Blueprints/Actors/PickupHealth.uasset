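; PickupHealth is a health pickup that gives one health to a TopDownCharacter.
; It supplies the PickupCondition check, which passes only while the character's Health is below MaxHealth, and the DoAbility event, which calls AddOneHealth through a DoOnce so it fires a single time.
; Tick runs the parent logic, then spins the static mesh around its pitch axis, scaled by delta time and the Rotation variable.
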(event EventBeginPlay
  (|CallParentFunction) ; This node is disabled and will not be called.\nDrag off pins to build functionality.
)

(event EventTick
  (params (DeltaSeconds :type Float%20%28single-precision%29))
  (|CallParentFunction DeltaSeconds)
  (Transformation|AddLocalRotation (Variables|Default|GetStaticMesh) (Math|Rotator|MakeRotator 0.0 (* DeltaSeconds (Variables|Default|GetRotation)) 0.0) false false))

(event EventDoAbility
  (params (Actor :type Actor%20Object%20Reference))
  (Utilities|FlowControl|DoOnce false
    (:Completed
      (bind _astop_down_character (Utilities|Casting|CastToTopDownCharacter Actor))
      (Default|AddOneHealth _astop_down_character))))

(fn ConstructionScript
  (|CallParentFunction))

(fn PickupCondition
  (params (Actor :type Actor%20Object%20Reference))
  (bind _astop_down_character (Utilities|Casting|CastToTopDownCharacter Actor))
  (return (< (Variables|/Game/Blueprints/Character/TopDownCharacter.TopDownCharacter_C|GetHealth _astop_down_character) (Variables|/Game/Blueprints/Character/TopDownCharacter.TopDownCharacter_C|GetMaxHealth _astop_down_character))))