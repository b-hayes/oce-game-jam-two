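; Base pickup actor that grants an ability to a TopDownCharacter that overlaps it.
; On BeginPlay it plays a spatialized power-up sound at its Sphere component's location.
; The first character overlap passes a DoOnce gate, then on authority only sets the character's AbilityBase current ability to AbilityToGrant and destroys the pickup.
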(event EventBeginPlay
  (Audio|SpawnSoundatLocation "/Game/Audio/SFX/478336__joao-janz__bouncing-power-up-1-3.478336__joao-janz__bouncing-power-up-1-3" (Transformation|GetWorldLocation (Variables|Default|GetSphere)) "0, 0, 0" 1.0 1.0 0.0 "/Game/Audio/Settings/CloseSounds.CloseSounds" 0))

(event Collision|EventActorBeginOverlap
  (params (OtherActor :type Actor%20Object%20Reference))
  (bind _astop_down_character (Utilities|Casting|CastToTopDownCharacter OtherActor))
  (Utilities|FlowControl|DoOnce false
    (:Completed
      (Networking|SwitchHasAuthority
        (:Authority
          (Variables|/Game/Blueprints/Components/AbilityComponent.AbilityComponent_C|SetCurrentAbility (Variables|/Game/Blueprints/Character/TopDownCharacter.TopDownCharacter_C|GetAbilityBase _astop_down_character) (Variables|Default|GetAbilityToGrant))
          (Actor|DestroyActor))))))

(event EventTick
  (params (DeltaSeconds :type Float%20%28single-precision%29)))

(fn ConstructionScript)