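; Proximity mine actor that damages TopDownCharacters within its capsule when triggered.
; On BeginPlay a Timeline lowers the sphere out of its initial position, then after a short delay enables query-only collision on the capsule to arm it.
; Overlap events track characters in an InRadius list.
; The first overlap resets the sphere's position, waits a configurable fuse, spawns the explosion effect, damages everyone still in range and destroys the mine.
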(event OnComponentBeginOverlap(Capsule)
  (params (OverlappedComponent :type Primitive%20Component%20Object%20Reference) (OtherActor :type Actor%20Object%20Reference) (OtherComp :type Primitive%20Component%20Object%20Reference) (OtherBodyIndex :type Integer) (bFromSweep :type Boolean) (SweepResult :type Hit%20Result%20Structure%20%28by%20ref%29))
  (bind _astop_down_character (Utilities|Casting|CastToTopDownCharacter OtherActor))
  (Utilities|Array|AddUnique (Variables|Default|GetInRadius) _astop_down_character)
  (Utilities|FlowControl|DoOnce false
    (:Completed
      (Transformation|SetRelativeLocation (Variables|Default|GetSphere) "0, 0, 0" false false)
      (Utilities|FlowControl|Delay (Variables|Default|GetBombDelayBeforeExplosion))
      (Niagara|SpawnSystematLocation "/Game/Blueprints/Particles/BombExplosion_System.BombExplosion_System" (Transformation|GetActorLocation))
      (for _array_element (Variables|Default|GetInRadius)
        (Default|DamageCharacter _array_element 1))
      (Actor|DestroyActor))))

(event OnComponentEndOverlap(Capsule)
  (params (OverlappedComponent :type Primitive%20Component%20Object%20Reference) (OtherActor :type Actor%20Object%20Reference) (OtherComp :type Primitive%20Component%20Object%20Reference) (OtherBodyIndex :type Integer))
  (bind _astop_down_character (Utilities|Casting|CastToTopDownCharacter OtherActor))
  (Utilities|Array|RemoveItem (Variables|Default|GetInRadius) _astop_down_character))

(event EventBeginPlay
  (bind _percent (Timeline|Timeline_0 Play)
    (:Update
      (Transformation|SetRelativeLocation (Variables|Default|GetSphere) (Math|Vector|Lerp(Vector) (Variables|Default|GetInitialLocation) "0, 0,-500.000000" _percent) false false))
    (:Finished
      (Utilities|FlowControl|Delay 1.0)
      (Collision|SetCollisionEnabled (Variables|Default|GetCapsule) "QueryOnly"))))

(fn ConstructionScript)