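; PickupStand is an actor that spawns a random pickup at its spawn location, with all spawning restricted to the network authority.
; After an initial delay on BeginPlay, it picks a class from PickupOptions and stores the spawned actor, owned by the stand, as CurrentPickup.
; StartItemSpawnTimer waits for the respawn delay, then reuses the same spawn path, which spawns only if no valid pickup exists.
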(event Custom|StartItemSpawnTimer
  (Networking|SwitchHasAuthority
    (:Authority
      (Utilities|FlowControl|Delay (Variables|Default|GetItemSpawnTimer))
      (Utilities|IsValid (Variables|Default|GetCurrentPickup)
        (:Is%20Not%20Valid
          (bind _returnvalue (Game|SpawnActorfromClass (Utilities|Array|Get(acopy) (Variables|Default|GetPickupOptions) (Math|Random|RandomIntegerinRange 0 (- (Utilities|Array|Length (Variables|Default|GetPickupOptions)) 1))) (Math|Conversions|ToTransform(Vector) (Transformation|GetWorldLocation (Variables|Default|GetPickupSpawnLocation))) "Undefined" self 0))
          (Variables|Default|SetCurrentPickup _returnvalue))))))

(event EventBeginPlay
  (Networking|SwitchHasAuthority
    (:Authority
      (Utilities|FlowControl|Delay (Variables|Default|GetDelayBeforeInitialSpawn))
      (Utilities|IsValid (Variables|Default|GetCurrentPickup)
        (:Is%20Not%20Valid
          (bind _returnvalue (Game|SpawnActorfromClass (Utilities|Array|Get(acopy) (Variables|Default|GetPickupOptions) (Math|Random|RandomIntegerinRange 0 (- (Utilities|Array|Length (Variables|Default|GetPickupOptions)) 1))) (Math|Conversions|ToTransform(Vector) (Transformation|GetWorldLocation (Variables|Default|GetPickupSpawnLocation))) "Undefined" self 0))
          (Variables|Default|SetCurrentPickup _returnvalue))))))

(event Collision|EventActorBeginOverlap
  (params (OtherActor :type Actor%20Object%20Reference)))

(event EventTick
  (params (DeltaSeconds :type Float%20%28single-precision%29)))

(fn ConstructionScript)